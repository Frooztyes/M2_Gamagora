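; BP_Abe is the player character, a mage who casts spells made of boid swarms and tracks score on a HUD.
; Left click launches a small electric orb swarm; holding right grows an explosive fireball boid by boid, launched on release before a HUD-driven cooldown.
; Both spawn a BoidGenerator at the hand, aimed by a camera-direction trace running from far away back to the hand.
; Tick feeds movement speed to the reticle for cursor sizing.
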(event `self.ReceiveBeginPlay`
  (bind _returnvalue (`|CreateWidget` "/Game/UI/Reticle.Reticle_C"))
  (bind _output_get (set `self.Reticle` _returnvalue))
  (`UserWidget.AddToViewport` _output_get 0)
  (set `/Game/UI/Reticle.CharacterMovement` (`self.CharacterMovement`) _output_get)
  (bind _returnvalue_2 (`|CreateWidget` "/Game/HUD/HUD.HUD_C"))
  (`UserWidget.AddToViewport` _returnvalue_2 0)
  (bind _output_get_2 (set `self.hud` _returnvalue_2))
  (`/Game/HUD/HUD.ChangeScore` _output_get_2 (`self.score`)))

(event `self.ReceiveTick`
  (params (DeltaSeconds :type "Float (single-precision)"))
  (bind _reticle (`self.Reticle`))
  (bind _currentfireball (`self.currentFireball`))
  (set `/Game/UI/Reticle.PlayerSpeed` (`KismetMathLibrary.VSize` (`MovementComponent.Velocity` (`self.CharacterMovement`))) _reticle)
  (`/Game/UI/Reticle.ChangeCursorSize` _reticle)
  (if (`self.RightIsHold`)
    (`/Engine/EditorBlueprintResources/StandardMacros.DoOnce` false :!label _label
      (:`Completed`
        (bind _returnvalue (`BoidGenerator.GetBoidsNumber` _currentfireball))
        (if (<= _returnvalue (`self.maxFireballBoids`))
          (bind _returnvalue_2 (`BoidGenerator.AddBoid` _currentfireball true))
          (`NiagaraFunctionLibrary.SpawnSystemAttached` "/Game/Particles/NiagaraSystem/NS_FireSimulation.NS_FireSimulation" (`self.GetComponentByClass` _returnvalue_2 "/Script/Engine.StaticMeshComponent") "None" (0.0 0.0 0.0) (struct) "SnapToTarget" true)
          (bind _returnvalue_3 (`BoidGenerator.GetBoidsNumber` (`self.currentFireball`)))
          (`/Game/HUD/HUD.AddFireball` (`self.hud`) _returnvalue_3)
          (`KismetSystemLibrary.Delay` 1.0)
          (goto _label :!via `Reset`))))))

(event `Key|LeftMouseButton`
  (params (Key :type "Key Structure"))
  (bind _currentfireball (`self.currentFireball`))
  (:`Pressed`
    (if (not (`self.RightIsHold`))
      (`/Engine/EditorBlueprintResources/StandardMacros.DoOnce` false :!label _label_2
        (:`Completed`
          (set `self.LeftIsHold` true)
          (`self.PlayAnimMontage` "/Game/Characters/Abe/Animations/Attack_1Hand.Attack_1Hand")
          (bind _boidgenerator (`self.CreateFireball` 4 "/Engine/BasicShapes/Sphere.Sphere" "/Game/Materials/BlackOrb.BlackOrb" true (`self.FireballPosition`)))
          (set `self.currentFireball` _boidgenerator)
          (`KismetSystemLibrary.Delay` 0.5)
          (bind (_start _end) (`self.Get Shooting Direction` 9999999.0))
          (bind (_outhit _returnvalue) (`KismetSystemLibrary.LineTraceSingle` _start _end "TraceTypeQuery1" true (`self.actorsToIgnore`)))
          (if _returnvalue
            (`BoidGenerator.Launch` _currentfireball (`.Location` (`GameplayStatics.BreakHitResult` _outhit)))
            (else
              (`BoidGenerator.Launch` _currentfireball (* (- _start _end) 100000.0))))
          (`KismetSystemLibrary.Delay` 0.5)
          (goto _label_2 :!via `Reset`)))))
  (:`Released`
    (set `self.LeftIsHold` false)))

(event `Key|RightMouseButton`
  (params (Key :type "Key Structure"))
  (bind _currentfireball (`self.currentFireball`))
  (:`Pressed`
    (if (`self.LeftIsHold`)
      _
      (elif (`/Game/HUD/HUD.canRecast` (`self.hud`))
        (`/Engine/EditorBlueprintResources/StandardMacros.DoOnce` false :!label _label_3
          (:`Completed`
            (set `self.RightIsHold` true)
            (`self.PlayAnimMontage` "/Game/Characters/Abe/Animations/Standing_2H_Magic_Attack_01_Half_Montage.Standing_2H_Magic_Attack_01_Half_Montage")
            (bind (_boidgenerator _boids) (`self.CreateFireball` 3 "/Engine/BasicShapes/Plane.Plane" "/Game/Materials/Transparent.Transparent" false (`self.FireballPosition`)))
            (`/Game/HUD/HUD.AddFireball` (`self.hud`) (`KismetArrayLibrary.Array_Length` _boids))
            (set `self.currentFireball` _boidgenerator)
            (goto _label_4 :!via `Reset`))))))
  (:`Released`
    (`/Engine/EditorBlueprintResources/StandardMacros.DoOnce` true :!label _label_4
      (:`Completed`
        (`self.PlayAnimMontage` "/Game/Characters/Abe/Animations/Standing_2H_Magic_Attack_01_HalfOut_Montage.Standing_2H_Magic_Attack_01_HalfOut_Montage")
        (set `self.RightIsHold` false)
        (bind (_start _end) (`self.Get Shooting Direction` 9999999.0))
        (bind (_outhit _returnvalue) (`KismetSystemLibrary.LineTraceSingle` _start _end "TraceTypeQuery1" true (`self.actorsToIgnore`)))
        (if _returnvalue
          (`BoidGenerator.Launch` _currentfireball (`.Location` (`GameplayStatics.BreakHitResult` _outhit)))
          (else
            (`BoidGenerator.Launch` _currentfireball (* (- _start _end) 100000.0))))
        (`/Game/HUD/HUD.IsReloading` (`self.hud`) (`self.fireballCooldown`))
        (`/Game/HUD/HUD.AddFireball` (`self.hud`) 0)
        (goto _label_3 :!via `Reset`)))))

(event `AddPoint`
  (params (value :type Integer))
  (bind _output_get (set `self.score` (+ value (`self.score`))))
  (`/Game/HUD/HUD.ChangeScore` (`self.hud`) _output_get))

(fn `CreateFireball`
  (params (NumBoids :type Integer) (StaticMesh :type "StaticMesh Object Reference") (Material :type "Material Object Reference") (estElectrique :type Boolean) (handPosition :type "SceneComponent Object Reference"))
  (returns (BoidGenerator :type "BoidGenerator Object Reference") (boids :type "Array of Boids Object Reference"))
  (bind _returnvalue (`|SpawnActorFromClass` "/Script/Boid.BoidGenerator" (`SceneComponent.K2_GetComponentToWorld` handPosition) "Undefined" "MultiplyWithRoot" null null))
  (bind _returnvalue_2 (`BoidGenerator.Initialize` _returnvalue Material NumBoids StaticMesh (- (`SceneComponent.K2_GetComponentLocation` handPosition) (`SceneComponent.K2_GetComponentLocation` (`self.CapsuleComponent`))) "/Game/Particles/NiagaraSystem/NS_MagicOrb01.NS_MagicOrb01" 1000.0 35.0 10.0 50.0 15.0 (not estElectrique)))
  (for _array_element _returnvalue_2
    (if estElectrique
      (bind _returnvalue_3 (`self.GetComponentByClass` _array_element "/Script/Engine.StaticMeshComponent"))
      (`NiagaraFunctionLibrary.SpawnSystemAttached` "/Game/Particles/NiagaraSystem/NS_MagicOrb01.NS_MagicOrb01" _returnvalue_3 "None" (0.0 0.0 0.0) (struct) "SnapToTarget" true)
      (`self.SetActorScale3D` _array_element (0.2 0.2 0.2))
      (else
        (`NiagaraFunctionLibrary.SpawnSystemAttached` "/Game/Particles/NiagaraSystem/NS_FireSimulation.NS_FireSimulation" _returnvalue_3 "None" (0.0 0.0 0.0) (struct) "SnapToTarget" true))))
  (return _returnvalue _returnvalue_2))

(fn `Destroy Fireball After Timeout`
  (params (boid :type "Boids Object Reference"))
  (`self.K2_DestroyActor` boid))

(fn `Get Shooting Direction`
  (params (Range :type "Float (double-precision)"))
  (returns (Start :type "Vector Structure") (End :type "Vector Structure"))
  (bind _returnvalue (`SceneComponent.K2_GetComponentLocation` (`self.FireballPosition`)))
  (return (+ _returnvalue (* (`KismetMathLibrary.GetForwardVector` (`SceneComponent.K2_GetComponentRotation` (`self.FollowCamera`))) Range)) _returnvalue))

(fn `UserConstructionScript`)